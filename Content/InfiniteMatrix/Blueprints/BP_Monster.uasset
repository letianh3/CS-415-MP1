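; BP_Monster is an enemy that fires bullets, moves along a path and can hurt or be shot by the player.
; On BeginPlay it spawns a BP_MonsterBullet immediately and then every second, while the Move timeline drives its world Y position.
; Capsule overlap with BP_Player deals damage, shakes the camera, destroys the monster and handles player death with a restart display.
; Overlap with BP_Bullet destroys it and adds score.
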(event `self.ReceiveBeginPlay`
  (bind (_returnvalue_x _returnvalue_y _returnvalue_z) (`KismetMathLibrary.BreakVector` (`self.K2_GetActorLocation`)))
  (`|ExecutionSequence`
    (:`then_1`
      (`KismetSystemLibrary.K2_SetTimerDelegate` (delegate `自定义事件_0`) 1.0 true)
      (`|SpawnActorFromClass` "/Game/InfiniteMatrix/Blueprints/BP_MonsterBullet.BP_MonsterBullet_C" (`KismetMathLibrary.MakeTransform` (`SceneComponent.K2_GetComponentLocation` (`self.Scene`))) "AlwaysSpawn" "OverrideRootScale" null null :!label _label))
    (:`then_2`
      (bind (_direction _floor) (`Timeline|Move` :!via `PlayFromStart`)
        (:`Update`
          (`self.K2_SetActorLocation` (`KismetMathLibrary.MakeVector` _returnvalue_x _floor _returnvalue_z) true))))))

(event `自定义事件_0`
  (goto _label))

(event `self.Capsule.OnComponentBeginOverlap`
  (params (OverlappedComponent :type "PrimitiveComponent Object Reference") (OtherActor :type "Actor Object Reference") (OtherComp :type "PrimitiveComponent Object Reference") (OtherBodyIndex :type Integer) (bFromSweep :type Boolean) (SweepResult :type "HitResult Structure (by ref)"))
  (bind _asbp_player (cast `/Game/InfiniteMatrix/Blueprints/BP_Player` OtherActor)
    (:`then`
      (bind _health (`/Game/InfiniteMatrix/Blueprints/BP_Player.Health` _asbp_player))
      ;[1 1 1] 如果被玩家碰撞，则对玩家造成伤害并且销毁自身
      (set `/Game/InfiniteMatrix/Blueprints/BP_Player.Health` (- _health (`self.Damage`)) _asbp_player)
      (`self.K2_DestroyActor`)
      (`PlayerCameraManager.StartCameraShake` :`self` (`GameplayStatics.GetPlayerCameraManager` 0) :`ShakeClass` "/Game/InfiniteMatrix/Blueprints/CameraShake.CameraShake_C" :`Scale` 3.0)
      (if (<= _health 0.0)
        (set `/Game/InfiniteMatrix/Blueprints/BP_Player.IsDead` true _asbp_player)
        (`self.DisableInput` (`GameplayStatics.GetPlayerController` 0) null)
        (`/Game/InfiniteMatrix/Blueprints/BP_Player.DisplayRestart` _asbp_player)))
    (:`CastFailed`
      ;[1 1 1] 如果被子弹击中，则销毁自身
      (cast `/Game/InfiniteMatrix/Blueprints/BP_Bullet` OtherActor)
      (`self.K2_DestroyActor`)
      (bind _asbp_player_2 (cast `/Game/InfiniteMatrix/Blueprints/BP_Player` (`GameplayStatics.GetPlayerPawn` 0)))
      (`/Game/InfiniteMatrix/Blueprints/BP_Player.AddScore` _asbp_player_2 1))))

(fn `UserConstructionScript`)