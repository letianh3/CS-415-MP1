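; BP_Tunnel is an endless-tunnel segment with a rotating holed wall that randomly spawns health and monster actors, removing them when destroyed.
; Crossing its trigger scores a point unless the player hit the wall, asks TunnelSpawner for another segment, then destroys this one.
; Wall hits deal random damage, shake the camera, recolor all tunnels by player health and handle death.
; RandomizeWall picks one of four hole meshes and a random roll.
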(event `self.ReceiveBeginPlay`
  (bind _box (`self.Box`))
  (bind _box_2 (`self.Box`))
  (`|ExecutionSequence`
    (:`then_0`
      (if (`self.HasGeneratedHealthBefore`)
        (set `self.HasGeneratedHealthBefore` false :!label _label)
        (elif (< (`KismetMathLibrary.RandomFloatInRange` 0.0 1.0) (`self.SpawnHealthProbability`))
          (goto _label)
          (else
            (bind _returnvalue (`|SpawnActorFromClass` "/Game/InfiniteMatrix/Blueprints/BP_Health.BP_Health_C" (`KismetMathLibrary.MakeTransform` (`KismetMathLibrary.RandomPointInBoundingBox` (`SceneComponent.K2_GetComponentLocation` _box) (`BoxComponent.GetScaledBoxExtent` _box))) "AlwaysSpawn" "OverrideRootScale" null null))
            (set `self.HasGeneratedHealthBefore` true)
            (`KismetArrayLibrary.Array_Add` (`self.SpawnHealths`) _returnvalue)))))
    (:`then_1`
      (if (`self.HasGeneratedMonsterBefore`)
        (set `self.HasGeneratedMonsterBefore` false :!label _label_2)
        (elif (< (`KismetMathLibrary.RandomFloatInRange` 0.0 1.0) (`self.SpawnMonsterProbability`))
          (goto _label_2)
          (else
            (for _ (range 1 (+ (`KismetMathLibrary.RandomIntegerInRange` 1 3) 1))
              (bind _returnvalue_2 (`|SpawnActorFromClass` "/Game/InfiniteMatrix/Blueprints/BP_Monster.BP_Monster_C" (`KismetMathLibrary.MakeTransform` (`KismetMathLibrary.RandomPointInBoundingBox` (`SceneComponent.K2_GetComponentLocation` _box_2) (`BoxComponent.GetScaledBoxExtent` _box_2))) "AdjustIfPossibleButDontSpawnIfColliding" "OverrideRootScale" null 5.0 null))
              (`KismetArrayLibrary.Array_Add` (`self.SpawnMonsters`) _returnvalue_2))
            (set `self.HasGeneratedMonsterBefore` true)))))))

(event `self.ReceiveTick`
  (params (DeltaSeconds :type "Float (single-precision)"))
  (`SceneComponent.K2_AddLocalRotation` (`self.WallMesh`) (`KismetMathLibrary.MakeRotator` (* DeltaSeconds (`self.RotateSpeed`))) false false))

(event `self.TriggerZone.OnComponentBeginOverlap`
  (params (OverlappedComponent :type "PrimitiveComponent Object Reference") (OtherActor :type "Actor Object Reference") (OtherComp :type "PrimitiveComponent Object Reference") (OtherBodyIndex :type Integer) (bFromSweep :type Boolean) (SweepResult :type "HitResult Structure (by ref)"))
  (bind _asbp_player (cast `/Game/InfiniteMatrix/Blueprints/BP_Player` OtherActor))
  ;[1 1 1] Increase score if not hitwall
  (if (not (`self.isHitWall?`))
    (set `/Game/InfiniteMatrix/Blueprints/BP_Player.Score` (+ (`/Game/InfiniteMatrix/Blueprints/BP_Player.Score` _asbp_player) 1) _asbp_player))
  (`/Game/InfiniteMatrix/Blueprints/BP_TunnelSpawner.SpawnTunnelAtSpawnPoint` (`self.TunnelSpawner`))
  (`self.K2_DestroyActor`))

(event `self.ReceiveDestroyed`
  (bind _spawnhealths (`self.SpawnHealths`))
  (for _array_element (`self.SpawnMonsters`)
    (`/Engine/EditorBlueprintResources/StandardMacros.IsValid` _array_element
      (:`Is Valid`
        (`self.K2_DestroyActor` _array_element))))
  (`KismetArrayLibrary.Array_Clear` (`self.SpawnMonsters`))
  (for _array_element_2 _spawnhealths
    (`/Engine/EditorBlueprintResources/StandardMacros.IsValid` _array_element_2
      (:`Is Valid`
        (`self.K2_DestroyActor` _array_element_2))))
  (`KismetArrayLibrary.Array_Clear` _spawnhealths))

(event `self.WallMesh.OnComponentBeginOverlap`
  (params (OverlappedComponent :type "PrimitiveComponent Object Reference") (OtherActor :type "Actor Object Reference") (OtherComp :type "PrimitiveComponent Object Reference") (OtherBodyIndex :type Integer) (bFromSweep :type Boolean) (SweepResult :type "HitResult Structure (by ref)"))
  (bind _asbp_player (cast `/Game/InfiniteMatrix/Blueprints/BP_Player` OtherActor)
    (:`then`
      (set `self.isHitWall?` true)
      (bind _output_get (set `/Game/InfiniteMatrix/Blueprints/BP_Player.Health` (- (`/Game/InfiniteMatrix/Blueprints/BP_Player.Health` _asbp_player) (`KismetMathLibrary.RandomFloatInRange` (`self.MinDamage`) (`self.MaxDamage`))) _asbp_player))
      (`PlayerCameraManager.StartCameraShake` :`self` (`GameplayStatics.GetPlayerCameraManager` 0) :`ShakeClass` "/Game/InfiniteMatrix/Blueprints/CameraShake.CameraShake_C" :`Scale` 3.0)
      (`self.SetWallColorFromPlayerHealth`)
      (if (<= _output_get 0.0)
        (set `/Game/InfiniteMatrix/Blueprints/BP_Player.IsDead` true _asbp_player)
        (`self.DisableInput` (`GameplayStatics.GetPlayerController` 0) null)
        (`/Game/InfiniteMatrix/Blueprints/BP_Player.DisplayRestart` _asbp_player)))
    (:`CastFailed`
      (set `self.isHitWall?` false))))

(fn `RandomizeWall`
  (`StaticMeshComponent.SetStaticMesh` (`self.WallMesh`) (select `int` (`KismetMathLibrary.RandomIntegerInRange` 0 3) :`0` "/Game/InfiniteMatrix/Meshes/SM_Hole_01.SM_Hole_01" :`1` "/Game/InfiniteMatrix/Meshes/SM_Hole_02.SM_Hole_02" :`2` "/Game/InfiniteMatrix/Meshes/SM_Hole_03.SM_Hole_03" :`3` "/Game/InfiniteMatrix/Meshes/SM_Hole_04.SM_Hole_04" :!type "StaticMesh Object Reference"))
  (`SceneComponent.K2_AddLocalRotation` (`self.WallMesh`) (`KismetMathLibrary.MakeRotator` (`KismetMathLibrary.RandomFloatInRange` 0.0 360.0)) false false))

(fn `SetWallColorFromPlayerHealth`
  (bind _outactors (`GameplayStatics.GetAllActorsOfClass` "BP_Tunnel_C"))
  (for _array_element _outactors
    (bind _returnvalue (`PrimitiveComponent.CreateDynamicMaterialInstance` (`/Game/InfiniteMatrix/Blueprints/BP_Tunnel.WallMesh` _array_element) 0 "/Game/InfiniteMatrix/Materials/MI_Hole.MI_Hole" "None"))
    (bind _asbp_player (cast `/Game/InfiniteMatrix/Blueprints/BP_Player` (`GameplayStatics.GetPlayerPawn` 0)))
    (bind _health (`/Game/InfiniteMatrix/Blueprints/BP_Player.Health` _asbp_player))
    (if (> _health 50.0)
      (set `self.WallColor` (struct :`G` 1.0 :`B` 0.286275 :`A` 1.0))
      (`MaterialInstanceDynamic.SetVectorParameterValue` _returnvalue "Color" (`self.WallColor`) :!label _label)
      (elif (< _health 50.0)
        (if (< _health 20.0)
          (set `self.WallColor` (struct :`R` 1.0 :`A` 1.0))
          (goto _label)
          (else
            (set `self.WallColor` (struct :`R` 1.0 :`G` 0.33023 :`A` 1.0))
            (goto _label)))))))

(fn `UserConstructionScript`)